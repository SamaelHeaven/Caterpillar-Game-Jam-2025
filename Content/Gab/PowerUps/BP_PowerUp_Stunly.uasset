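; Stunly power-up for the Caterpillar Slide game mode that gives the player a temporary speed boost.
; ActivatePowerUp stores the player, doubles its negative Speed value, then adds score through GM_CaterpillarSlide and plays a boost sound.
; It also starts a few-second timer, apparently bound to SetNormalSpeed, which sets a fixed normal speed rather than restoring the previous value.
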(event Custom|SetNormalSpeed
  (Variables|/Game/Samuel/BP_Player.BP_Player_C|SetSpeed (Variables|Default|GetPlayer) -1e+03))

(event EventBeginPlay
  (|CallParentFunction) ; This node is disabled and will not be called.\nDrag off pins to build functionality.
)

(event Collision|EventActorBeginOverlap
  (params (OtherActor :type Actor%20Object%20Reference))
  (|CallParentFunction OtherActor) ; This node is disabled and will not be called.\nDrag off pins to build functionality.
)

(event EventTick
  (params (DeltaSeconds :type Float%20%28single-precision%29))
  (|CallParentFunction DeltaSeconds) ; This node is disabled and will not be called.\nDrag off pins to build functionality.
)

(fn ConstructionScript
  (|CallParentFunction))

(fn ActivatePowerUp
  (params (Player :type BP%20Player%20Object%20Reference))
  (bind _output_get (Variables|Default|SetPlayer Player))
  (Variables|/Game/Samuel/BP_Player.BP_Player_C|SetSpeed _output_get -2e+03)
  (bind _asgm_caterpillar_slide (Utilities|Casting|CastToGM_CaterpillarSlide (Game|GetGameMode)))
  (Default|IncreaseScore _asgm_caterpillar_slide 100)
  (Audio|PlaySound2D "/Game/Simon/sounds/stunly_boost.stunly_boost" 1.0 1.0 0.0 0 0)
  (Utilities|Time|SetTimerbyEvent (EventDispatchers|CreateEvent :!event Custom|SetNormalSpeed) 5.0))