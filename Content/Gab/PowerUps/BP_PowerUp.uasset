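; BP_PowerUp is a pickup actor that gives itself to the player as a power-up.
; When a BP_Player overlaps its mesh, it plays a 2D pickup sound and passes itself to the player's BPCPowerUpHandler component.
; It then hides the mesh and disables its overlaps instead of destroying the actor, so the handler's reference stays valid.
; ActivatePowerUp is an empty function, so this Blueprint defines no effect of its own.
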(event OnComponentBeginOverlap(Mesh)
  (params (OverlappedComponent :type Primitive%20Component%20Object%20Reference) (OtherActor :type Actor%20Object%20Reference) (OtherComp :type Primitive%20Component%20Object%20Reference) (OtherBodyIndex :type Integer) (bFromSweep :type Boolean) (SweepResult :type Hit%20Result%20Structure%20%28by%20ref%29))
  (bind _asbp_player (Utilities|Casting|CastToBP_Player OtherActor))
  (Audio|PlaySound2D "/Game/Simon/sounds/pickup-sound.pickup-sound" 1.0 1.0 0.0 0 0)
  (CallFunction|AddPowerUptoPlayer _asbp_player)
  (Rendering|SetVisibility (Variables|Default|GetMesh) false false)
  (Variables|/Script/Engine.PrimitiveComponent|SetbGenerateOverlapEvents (Variables|Default|GetMesh) false))

(event EventBeginPlay
  (|CallParentFunction) ; This node is disabled and will not be called.\nDrag off pins to build functionality.
)

(event Collision|EventActorBeginOverlap
  (params (OtherActor :type Actor%20Object%20Reference))
  (|CallParentFunction OtherActor) ; This node is disabled and will not be called.\nDrag off pins to build functionality.
)

(event EventTick
  (params (DeltaSeconds :type Float%20%28single-precision%29))
  (|CallParentFunction DeltaSeconds) ; This node is disabled and will not be called.\nDrag off pins to build functionality.
)

(fn ConstructionScript
  (|CallParentFunction))

(fn AddPowerUptoPlayer
  (params (Player :type BP%20Player%20Object%20Reference))
  (Default|SetPowerUp (Variables|/Game/Samuel/BP_Player.BP_Player_C|GetBPC_PowerUpHandler Player) self))

(fn ActivatePowerUp
  (params (Player :type BP%20Player%20Object%20Reference)))