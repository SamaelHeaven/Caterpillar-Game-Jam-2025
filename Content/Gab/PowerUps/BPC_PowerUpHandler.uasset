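; BPC_PowerUpHandler is a component on BP_Player that holds one power-up at a time and lets the player use it.
; SetPowerUp stores the power-up and fires an OnSetPowerUp call with its image.
; Pressing E runs ActivatePowerUp, which activates the held power-up on the cached owning player, clears the slot and fires an OnRemovePowerUp call.
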(event EventBeginPlay
  (bind _asbp_player (Utilities|Casting|CastToBP_Player (Components|GetOwner)))
  (Variables|Default|SetPlayer _asbp_player))

(event Input|KeyboardEvents|E
  (params (Key :type Key%20Structure))
  (:Pressed
    (CallFunction|ActivatePowerUp)))

(fn SetPowerUp
  (params (PowerUp :type BP%20Power%20Up%20Object%20Reference))
  (bind _output_get (Variables|Default|SetPowerUp PowerUp))
  (Default|CallOnSetPowerUp (Variables|/Game/Gab/PowerUps/BP_PowerUp.BP_PowerUp_C|GetImage _output_get)))

(fn ActivatePowerUp
  (bind _powerup (Variables|Default|GetPowerUp)
    (:then
      (Default|ActivatePowerUp _powerup (Variables|Default|GetPlayer))
      (Variables|Default|SetPowerUp 0)
      (Default|CallOnRemovePowerUp))
    (:else)))