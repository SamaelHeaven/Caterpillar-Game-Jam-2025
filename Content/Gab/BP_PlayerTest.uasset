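; Test player pawn for an auto-forward physics runner in which leaf count serves as health.
; Tick forces the skeletal mesh's Y velocity to Speed, applies X impulses while Left/A or Right/D is held, and moves the spring arm along Y and Z only.
; Space adds an upward impulse.
; Branch overlaps disable that branch's overlaps, knock the player against its X velocity and cost leaves, firing leaf-decrease dispatchers.
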(event Custom|On%20Hit%20By%20Branch
  (params (Branch :type BP%20Branch%20Object%20Reference))
  (CallFunction|DecreaseHealth 4.0)
  (Variables|/Script/Engine.PrimitiveComponent|SetbGenerateOverlapEvents (Variables|/Game/Samuel/BP_Branch.BP_Branch_C|GetStaticMesh Branch) false)
  (bind _returnvalue (Physics|GetPhysicsLinearVelocity (Variables|Default|GetSkeletalMesh) "None"))
  (if (< (.x _returnvalue) 0.0)
    (Physics|AddImpulse (Variables|Default|GetSkeletalMesh) (Math|Vector|MakeVector (Variables|Default|GetBranchHitStrenght) 0.0 0.0) "None" true)
    (else
      (Physics|AddImpulse (Variables|Default|GetSkeletalMesh) (Math|Vector|MakeVector (* (Variables|Default|GetBranchHitStrenght) -1.0) 0.0 0.0) "None" true))))

(event Collision|EventActorBeginOverlap
  (params (OtherActor :type Actor%20Object%20Reference))
  (bind _asbp_branch (Utilities|Casting|CastToBP_Branch OtherActor))
  (CallFunction|OnHitbyBranch _asbp_branch))

(event EventTick
  (params (DeltaSeconds :type Float%20%28single-precision%29))
  (bind _springarm (Variables|Default|GetSpringArm))
  (bind _skeletalmesh (Variables|Default|GetSkeletalMesh))
  (bind _skeletalmesh_2 (Variables|Default|GetSkeletalMesh))
  (bind _returnvalue (Transformation|GetWorldLocation _skeletalmesh))
  (Utilities|FlowControl|Sequence
    (:then_0
      (bind _returnvalue_2 (Physics|GetPhysicsLinearVelocity _skeletalmesh_2 "None"))
      (Physics|SetPhysicsLinearVelocity _skeletalmesh_2 (Math|Vector|MakeVector (.x _returnvalue_2) (Variables|Default|GetSpeed) (.z _returnvalue_2)) false "None"))
    (:then_1
      (Transformation|SetWorldLocation _springarm (Math|Vector|MakeVector (.x (Transformation|GetWorldLocation _springarm)) (+ (.y _returnvalue) (Variables|Default|GetSpringArmOffsetY)) (+ (.z _returnvalue) (Variables|Default|GetSpringArmOffsetZ))) false false)
      (if (and (not (Variables|Default|GetIsRightPressed)) (Variables|Default|GetIsLeftPressed))
        (Physics|AddImpulse (Variables|Default|GetSkeletalMesh) (Math|Vector|MakeVector (* (Variables|Default|GetTurnPower) -1.0) 0.0 0.0) "None" true)
        (elif (and (Variables|Default|GetIsRightPressed) (not (Variables|Default|GetIsLeftPressed)))
          (Physics|AddImpulse (Variables|Default|GetSkeletalMesh) (Math|Vector|MakeVector (Variables|Default|GetTurnPower) 0.0 0.0) "None" true))))))

(event Input|KeyboardEvents|SpaceBar
  (params (Key :type Key%20Structure :default "None"))
  (:Pressed
    (Physics|AddImpulse (Variables|Default|GetSkeletalMesh) "0.000000,0.000000,2500.000000" "None" true)))

(event Input|KeyboardEvents|Left
  (params (Key :type Key%20Structure :default "None"))
  (:Pressed
    (Variables|Default|SetIsLeftPressed true))
  (:Released
    (Variables|Default|SetIsLeftPressed false)))

(event Input|KeyboardEvents|Right
  (params (Key :type Key%20Structure :default "None"))
  (:Pressed
    (Variables|Default|SetIsRightPressed true))
  (:Released
    (Variables|Default|SetIsRightPressed false)))

(event Input|KeyboardEvents|A
  (params (Key :type Key%20Structure :default "None"))
  (:Pressed
    (Variables|Default|SetIsLeftPressed true))
  (:Released
    (Variables|Default|SetIsLeftPressed false)))

(event Input|KeyboardEvents|D
  (params (Key :type Key%20Structure :default "None"))
  (:Pressed
    (Variables|Default|SetIsRightPressed true))
  (:Released
    (Variables|Default|SetIsRightPressed false)))

(fn ConstructionScript)

(fn IncreaseLeafCount
  (Math|Float|IncrementFloat (Variables|Health|GetLeafCount)
    (:%20%20
      (Default|CallOnLeafIncrease))))

(fn DecreaseLeafCount
  (Math|Float|DecrementFloat (Variables|Health|GetLeafCount)
    (:%20%20
      (Default|CallOnLeafDecrease))))

(fn DecreaseHealth
  (params (LeafCount :type Float%20%28double-precision%29))
  (for _index (range 0 (- (Math|Float|Truncate LeafCount) 1))
    (Default|CallOnLeafDecrease))
  (Variables|Health|SetLeafCount (- (Variables|Health|GetLeafCount) LeafCount)))