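; Player actor for a dodging game, driven forward at constant speed along Y while A/D or arrow keys steer it sideways.
; Tick sets the physics mesh's velocity, applies turn impulses and moves the spring arm to follow on Y and Z.
; Branch hits consume a shield or flash red, cost health and knock the player sideways.
; BP_Death overlaps or depleted health freeze physics and swap the HUD for game over.
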(event Custom|On%20Hit%20By%20Branch
  (params (Branch :type BP%20Branch%20Object%20Reference))
  (bind _skeletalmesh (Variables|Default|GetSkeletalMesh))
  (if (Variables|Default|GetIsProtected)
    (Variables|Default|SetIsProtected false)
    (Rendering|SetVisibility (Variables|Default|GetShieldMesh) false false)
    (Audio|PlaySound2D "/Game/Simon/sounds/shield_protection.shield_protection" 1.0 1.0 0.0 0 0)
    (else
      (Rendering|Material|SetMaterial _skeletalmesh 0 "/Game/Hugo/Materials/M_Color_Red.M_Color_Red")
      (Utilities|FlowControl|Delay 0.2)
      (Rendering|Material|SetMaterial _skeletalmesh 0 "/Game/Fred/Butter/Material_008.Material_008")
      (Audio|PlaySound2D "/Game/Simon/sounds/hit-sound.hit-sound" 1.0 1.0 0.0 0 0)
      (CallFunction|DecreaseHealth 1)
      (Variables|/Script/Engine.PrimitiveComponent|SetbGenerateOverlapEvents (Variables|/Game/Samuel/BP_Branch.BP_Branch_C|GetStaticMesh Branch) false)
      (bind _returnvalue (Physics|GetPhysicsLinearVelocity (Variables|Default|GetSkeletalMesh) "None"))
      (if (< (.x _returnvalue) 0.0)
        (Physics|AddImpulse (Variables|Default|GetSkeletalMesh) (Math|Vector|MakeVector (Variables|Default|GetBranchHitStrenght) 0.0 0.0) "None" true)
        (else
          (Physics|AddImpulse (Variables|Default|GetSkeletalMesh) (Math|Vector|MakeVector (* (Variables|Default|GetBranchHitStrenght) -1.0) 0.0 0.0) "None" true))))))

(event Collision|EventActorBeginOverlap
  (params (OtherActor :type Actor%20Object%20Reference))
  (bind _asbp_branch (Utilities|Casting|CastToBP_Branch OtherActor)
    (:then
      (CallFunction|OnHitbyBranch _asbp_branch))
    (:CastFailed
      (Utilities|Casting|CastToBP_Death OtherActor)
      (CallFunction|Death))))

(event EventBeginPlay
  (bind _returnvalue (UserInterface|CreateWidget "/Game/Carlos/UI/WBP_MainHUD.WBP_MainHUD_C" (Game|GetPlayerController 0)))
  (bind _output_get (Variables|Default|SetHUD _returnvalue))
  (UserInterface|Viewport|AddtoViewport _output_get 0))

(event EventTick
  (params (DeltaSeconds :type Float%20%28single-precision%29))
  (bind _springarm (Variables|Default|GetSpringArm))
  (bind _skeletalmesh (Variables|Default|GetSkeletalMesh))
  (bind _skeletalmesh_2 (Variables|Default|GetSkeletalMesh))
  (bind _returnvalue (Transformation|GetWorldLocation _skeletalmesh))
  (if (not (Variables|Default|GetIsDead))
    (Utilities|FlowControl|Sequence
      (:then_0
        (bind _returnvalue_2 (Physics|GetPhysicsLinearVelocity _skeletalmesh_2 "None"))
        (Physics|SetPhysicsLinearVelocity _skeletalmesh_2 (Math|Vector|MakeVector (.x _returnvalue_2) (Variables|Default|GetSpeed) (.z _returnvalue_2)) false "None"))
      (:then_1
        (Transformation|SetWorldLocation _springarm (Math|Vector|MakeVector (.x (Transformation|GetWorldLocation _springarm)) (+ (.y _returnvalue) (Variables|Default|GetSpringArmOffsetY)) (+ (.z _returnvalue) (Variables|Default|GetSpringArmOffsetZ))) false false)
        (if (and (not (Variables|Default|GetIsRightPressed)) (Variables|Default|GetIsLeftPressed))
          (Physics|AddImpulse (Variables|Default|GetSkeletalMesh) (Math|Vector|MakeVector (* (Variables|Default|GetTurnPower) -1.0) 0.0 0.0) "None" true)
          (elif (and (Variables|Default|GetIsRightPressed) (not (Variables|Default|GetIsLeftPressed)))
            (Physics|AddImpulse (Variables|Default|GetSkeletalMesh) (Math|Vector|MakeVector (Variables|Default|GetTurnPower) 0.0 0.0) "None" true)))))))

(event Input|KeyboardEvents|Left
  (params (Key :type Key%20Structure :default "None"))
  (:Pressed
    (if (not (Variables|Default|GetIsDead))
      (Variables|Default|SetIsLeftPressed true)))
  (:Released
    (if (not (Variables|Default|GetIsDead))
      (Variables|Default|SetIsLeftPressed false))))

(event Input|KeyboardEvents|Right
  (params (Key :type Key%20Structure :default "None"))
  (:Pressed
    (if (not (Variables|Default|GetIsDead))
      (Variables|Default|SetIsRightPressed true)))
  (:Released
    (if (not (Variables|Default|GetIsDead))
      (Variables|Default|SetIsRightPressed false))))

(event Input|KeyboardEvents|A
  (params (Key :type Key%20Structure :default "None"))
  (:Pressed
    (if (not (Variables|Default|GetIsDead))
      (Variables|Default|SetIsLeftPressed true)))
  (:Released
    (if (not (Variables|Default|GetIsDead))
      (Variables|Default|SetIsLeftPressed false))))

(event Input|KeyboardEvents|D
  (params (Key :type Key%20Structure :default "None"))
  (:Pressed
    (if (not (Variables|Default|GetIsDead))
      (Variables|Default|SetIsRightPressed true)))
  (:Released
    (if (not (Variables|Default|GetIsDead))
      (Variables|Default|SetIsRightPressed false))))

(fn ConstructionScript)

(fn DecreaseHealth
  (params (Health :type Integer))
  (bind _output_get (Variables|Health|SetHealth (- (Variables|Health|GetHealth) Health)))
  (if (<= _output_get 0)
    (CallFunction|Death)
    (else
      (Default|CallOnHealthDecrease (Variables|Health|GetHealth)))))

(fn Death
  (Variables|Default|SetIsDead true)
  (Physics|SetSimulatePhysics (Variables|Default|GetSkeletalMesh) false)
  (Viewport|RemoveAllWidgets)
  (bind _returnvalue (UserInterface|CreateWidget "/Game/Carlos/UI/WBP_GameOver.WBP_GameOver_C" (Game|GetPlayerController 0)))
  (UserInterface|Viewport|AddtoViewport _returnvalue 0))

(fn IncreaseHealth
  (params (Health :type Integer))
  (bind _output_get (Variables|Health|SetHealth (+ (Variables|Health|GetHealth) Health)))
  (Default|CallOnHealthIncrease _output_get))