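; Player controller that shows the boss HUD on begin play and handles the pause menu.
; IA_Pause or Enter toggles the menu, creating it lazily and switching input mode and mouse cursor between game and UI.
; The game pauses only when the menu is first created; the toggle never unpauses or re-pauses it.
; Debug keys 1 and 2 display the Game Over and Winner screens for testing.
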(event Input|EnhancedActionEvents|EnhancedInputActionIA_Pause
  (params (ActionValue :type Boolean) (ElapsedSeconds :type Float%20%28double-precision%29) (TriggeredSeconds :type Float%20%28double-precision%29) (InputAction :type Input%20Action%20Object%20Reference :default "/Game/Carlos/Inputs/Actions/IA_Pause.IA_Pause"))
  (:Completed
    (CallFunction|ToogleMainMenu)))

(event EventBeginPlay
  (bind _returnvalue (UserInterface|CreateWidget "/Game/Carlos/UI/WBP_MainHUDBoss.WBP_MainHUDBoss_C" (Game|GetPlayerController 0)))
  (Variables|Default|SetHudRef _returnvalue)
  (UserInterface|Viewport|AddtoViewport _returnvalue 0))

(event EventTick
  (params (DeltaSeconds :type Float%20%28single-precision%29)))

(event Input|KeyboardEvents|1
  (params (Key :type Key%20Structure :default "None"))
  ;[1 1 1] Test Buttons (Game Over and Winne Screen)
  (:Pressed
    (bind _returnvalue (UserInterface|CreateWidget "/Game/Carlos/UI/WBP_GameOver.WBP_GameOver_C"))
    (UserInterface|Viewport|AddtoViewport _returnvalue 0)))

(event Input|KeyboardEvents|Enter
  (params (Key :type Key%20Structure :default "None"))
  (:Pressed
    (CallFunction|ToogleMainMenu)))

(event Input|KeyboardEvents|2
  (params (Key :type Key%20Structure :default "None"))
  ;[1 1 1] Test Buttons (Game Over and Winne Screen)
  (:Pressed
    (bind _returnvalue (UserInterface|CreateWidget "/Game/Carlos/UI/WBP_Winner.WBP_Winner_C"))
    (UserInterface|Viewport|AddtoViewport _returnvalue 0)))

(fn ConstructionScript)

(fn ToogleMainMenu
  (Variables|Default|GetWB_GameMenu
    (:then
      (if (Widget|IsVisible (Variables|Default|GetWB_GameMenu))
        (Widget|SetVisibility (Variables|Default|GetWB_GameMenu) "Collapsed")
        (CallFunction|FocusGame)
        (else
          (Widget|SetVisibility (Variables|Default|GetWB_GameMenu) "Visible")
          (CallFunction|FocusWidget :!label _label))))
    (:else
      (bind _returnvalue (UserInterface|CreateWidget "/Game/Carlos/UI/WBP_PauseMenu.WBP_PauseMenu_C" self))
      (bind _output_get (Variables|Default|SetWB_GameMenu _returnvalue))
      (UserInterface|Viewport|AddtoViewport _output_get 0)
      (Game|SetGamePaused true)
      (goto _label))))

(fn FocusGame
  (Variables|Default|SetbShowMouseCursor false)
  (Input|SetInputModeGameOnly self false))

(fn FocusWidget
  (Variables|Default|SetbShowMouseCursor true)
  (Input|SetInputModeGameandUI self (Variables|Default|GetWB_GameMenu) "DoNotLock" true false))