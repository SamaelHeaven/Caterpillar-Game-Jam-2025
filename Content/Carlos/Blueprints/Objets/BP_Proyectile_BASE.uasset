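; Base projectile Blueprint that damages the actor it hits and charges the butterfly's special bar on bird hits.
; BeginPlay copies Speed into the ProjectileMovement initial and max speeds.
; Sphere overlaps with anything but the owner trigger Destruction, which applies BaseDamage and destroys the projectile.
; An exact BP_Bird class match also increments a BP_Butterfly owner's SpecialBar and refreshes its bar display.
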(event OnComponentBeginOverlap(Sphere)
  (params (OverlappedComponent :type Primitive%20Component%20Object%20Reference) (OtherActor :type Actor%20Object%20Reference) (OtherComp :type Primitive%20Component%20Object%20Reference) (OtherBodyIndex :type Integer) (bFromSweep :type Boolean) (SweepResult :type Hit%20Result%20Structure%20%28by%20ref%29))
  (if (!= OtherActor (Components|GetOwner))
    (CallFunction|Destruction OtherActor)))

(event Custom|Destruction
  (params (HitActor :type Actor%20Object%20Reference))
  (Game|Damage|ApplyDamage HitActor (Variables|Default|GetBase%20Damage) 0 0)
  (if (== (Utilities|GetClass HitActor) "/Game/Carlos/Blueprints/Characters/BP_Bird.BP_Bird_C")
    (bind _asbp_butterfly (Utilities|Casting|CastToBP_Butterfly (Components|GetOwner))
      (:then
        (bind _result (Math|Float|IncrementFloat (Variables|/Game/Carlos/Blueprints/Characters/BP_Butterfly.BP_Butterfly_C|GetSpecialBar _asbp_butterfly))
          (:%20%20
            (Default|UpdateSpecialBar (Variables|/Game/Carlos/Blueprints/Characters/BP_Butterfly.BP_Butterfly_C|GetSpecialBarRef _asbp_butterfly) _result (Variables|/Game/Carlos/Blueprints/Characters/BP_Butterfly.BP_Butterfly_C|GetMaxSpecialBar _asbp_butterfly)))))
      (:CastFailed
        _))
    (Actor|DestroyActor)
    (else
      (Actor|DestroyActor))))

(event EventBeginPlay
  (bind _projectilemovement (Variables|Default|GetProjectileMovement))
  (bind _speed (Variables|Default|GetSpeed))
  (Variables|/Script/Engine.ProjectileMovementComponent|SetInitialSpeed _projectilemovement _speed)
  (Variables|/Script/Engine.ProjectileMovementComponent|SetMaxSpeed _projectilemovement _speed))

(event Collision|EventActorBeginOverlap
  (params (OtherActor :type Actor%20Object%20Reference)))

(event EventTick
  (params (DeltaSeconds :type Float%20%28single-precision%29)))

(fn ConstructionScript)