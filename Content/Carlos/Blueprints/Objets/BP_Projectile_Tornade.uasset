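; Tornado projectile actor that damages what it hits and can itself be destroyed by damage.
; On BeginPlay it sets the ProjectileMovement initial and max speed from its Speed variable.
; Box overlaps ignore BP_Proyectile_1 instances and the owner; any other actor receives BaseDamage and the projectile destroys itself.
; Incoming damage reduces LifeProyectile, and the projectile is destroyed once that reaches zero.
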(event OnComponentBeginOverlap(Box)
  (params (OverlappedComponent :type Primitive%20Component%20Object%20Reference) (OtherActor :type Actor%20Object%20Reference) (OtherComp :type Primitive%20Component%20Object%20Reference) (OtherBodyIndex :type Integer) (bFromSweep :type Boolean) (SweepResult :type Hit%20Result%20Structure%20%28by%20ref%29))
  (if (not (== (Utilities|GetClass OtherActor) "/Game/Carlos/Blueprints/Objets/BP_Proyectile_1.BP_Proyectile_1_C"))
    (if (not (== OtherActor (Components|GetOwner)))
      (CallFunction|Destruction OtherActor))))

(event Custom|Destruction
  (params (HitActor :type Actor%20Object%20Reference))
  (Game|Damage|ApplyDamage HitActor (Variables|Default|GetBase%20Damage) 0 0)
  (Actor|DestroyActor))

(event EventBeginPlay
  (bind _projectilemovement (Variables|Default|GetProjectileMovement))
  (bind _speed (Variables|Default|GetSpeed))
  (Variables|/Script/Engine.ProjectileMovementComponent|SetInitialSpeed _projectilemovement _speed)
  (Variables|/Script/Engine.ProjectileMovementComponent|SetMaxSpeed _projectilemovement _speed))

(event Collision|EventActorBeginOverlap
  (params (OtherActor :type Actor%20Object%20Reference)))

(event EventTick
  (params (DeltaSeconds :type Float%20%28single-precision%29)))

(event Game|Damage|EventAnyDamage
  (params (Damage :type Float%20%28single-precision%29) (DamageType :type Damage%20Type%20Object%20Reference) (InstigatedBy :type Controller%20Object%20Reference) (DamageCauser :type Actor%20Object%20Reference))
  (Variables|Default|SetLifeProyectile (- (Variables|Default|GetLifeProyectile) Damage))
  (if (<= (Variables|Default|GetLifeProyectile) 0.0)
    (Actor|DestroyActor)))

(fn ConstructionScript)