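; Flying bird boss that attacks on a repeating timer, tracks its health in a HUD widget and shows a winner screen on death.
; Each tick of the timer randomly fires a feather projectile or starts a dash, which drives Y-axis movement out and back using delays.
; Collision overlaps deal physical damage and flip the vertical direction used by WalkHorizontally, which nothing in this graph calls.
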(event OnComponentBeginOverlap(CollisionDetector)
  (params (OverlappedComponent :type Primitive%20Component%20Object%20Reference) (OtherActor :type Actor%20Object%20Reference) (OtherComp :type Primitive%20Component%20Object%20Reference) (OtherBodyIndex :type Integer) (bFromSweep :type Boolean) (SweepResult :type Hit%20Result%20Structure%20%28by%20ref%29))
  (Variables|Default|SetDirectionVertical (* (Variables|Default|GetDirectionVertical) -1.0))
  (Game|Damage|ApplyDamage OtherActor (Variables|Default|GetPhysic%20Damage) 0 0))

(event Custom|WalkHorizontally
  (if (not (Variables|Default|GetPhysicAttack?))
    (Pawn|Input|AddMovementInput (Transformation|GetActorUpVector) (Variables|Default|GetDirectionVertical) false)))

(event Custom|Attack
  (switch int (Math|Random|RandomInteger 2)
    (:0
      (CallFunction|FireProyectile))
    (:1
      (if (not (Variables|Default|GetPhysicAttack?))
        (CallFunction|DashAttack)))
    (:2
      (CallFunction|FireProyectile))))

(event Custom|DashAttack
  (Variables|Default|SetPhysicAttack? true)
  (Development|PrintString "Dash Attack")
  (Variables|/Script/Engine.CharacterMovementComponent|SetMaxFlySpeed (Variables|Character|GetCharacterMovement) 1.5e+03)
  (Utilities|FlowControl|Delay 1.0)
  (Variables|Default|SetDirectionHorizontal -1.0)
  (Utilities|FlowControl|Delay 1.5)
  (Variables|Default|SetPhysicAttack? false)
  (Variables|Default|SetDirectionHorizontal 1.0)
  (Variables|/Script/Engine.CharacterMovementComponent|SetMaxFlySpeed (Variables|Character|GetCharacterMovement) 6e+02))

(event Custom|HandleDeath
  (bind _returnvalue (UserInterface|CreateWidget "/Game/Carlos/UI/WBP_Winner.WBP_Winner_C"))
  (UserInterface|Viewport|AddtoViewport _returnvalue 0))

(event EventBeginPlay
  (Utilities|FlowControl|Sequence
    (:then_0
      (Variables|Default|SetCurrentBossLife (Variables|Default|GetMaxBossLife)))
    (:then_1
      (bind _returnvalue (UserInterface|CreateWidget "/Game/Carlos/UI/WBP_LifeBoss.WBP_LifeBoss_C"))
      (Variables|Default|SetHudLifeBoss _returnvalue)
      (Default|UpdateBossLife _returnvalue (Variables|Default|GetCurrentBossLife) (Variables|Default|GetMaxBossLife))
      (UserInterface|Viewport|AddtoViewport _returnvalue 0))
    (:then_2
      (Pawn|Components|CharacterMovement|SetMovementMode (Variables|Character|GetCharacterMovement) "MOVE_Flying" 0)
      (Utilities|Time|SetTimerbyEvent (delegate Custom|Attack) 1.0 true true))))

(event Collision|EventActorBeginOverlap
  (params (OtherActor :type Actor%20Object%20Reference)))

(event EventTick
  (params (DeltaSeconds :type Float%20%28single-precision%29))
  (if (Variables|Default|GetPhysicAttack?)
    (Pawn|Input|AddMovementInput (Math|Vector|MakeVector 0.0 (Variables|Default|GetDirectionHorizontal) 0.0) 1.0 false)))

(event Game|Damage|EventAnyDamage
  (params (Damage :type Float%20%28single-precision%29) (DamageType :type Damage%20Type%20Object%20Reference) (InstigatedBy :type Controller%20Object%20Reference) (DamageCauser :type Actor%20Object%20Reference))
  (bind _output_get (Variables|Default|SetCurrentBossLife (- (Variables|Default|GetCurrentBossLife) Damage)))
  (Default|UpdateBossLife (Variables|Default|GetHudLifeBoss) _output_get (Variables|Default|GetMaxBossLife))
  (if (<= (Variables|Default|GetCurrentBossLife) 0.0)
    (Actor|DestroyActor)
    (CallFunction|HandleDeath)))

(fn ConstructionScript)

(fn FireProyectile
  (if (not (Variables|Default|GetPhysicAttack?))
    (Game|SpawnActorfromClass "/Game/Carlos/Blueprints/Objets/BP_Proyectile_Feather.BP_Proyectile_Feather_C" (Transformation|GetWorldTransform (Variables|Default|GetFireBallPos)) "AlwaysSpawn" "MultiplyWithRoot" (Components|GetOwner) 1e+03 1.0 0)))