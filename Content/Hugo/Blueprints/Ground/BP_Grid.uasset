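; BP_Grid is an actor that fills an area around its world location with a grid of randomly chosen elements at BeginPlay.
; PopulateGrid clears GridArray, then runs nested row and column loops, spawning a random AvailableElements class at each point and storing it in the array.
; Spacing divides the grid width and length by one less than the item counts, so elements reach both edges, with half-size offsets centering the layout.
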(event EventBeginPlay
  (Variables|Default|SetWorldLocation (Transformation|GetWorldLocation (Variables|Default|GetDefaultSceneRoot)))
  (CallFunction|PopulateGrid))

(event Collision|EventActorBeginOverlap
  (params (OtherActor :type Actor%20Object%20Reference)))

(event EventTick
  (params (DeltaSeconds :type Float%20%28single-precision%29)))

(fn ConstructionScript)

(fn PopulateGrid
  (bind _availableelements (Variables|Default|GetAvailableElements))
  (Utilities|Array|Clear (Variables|Default|GetGridArray))
  (LocalVariables|SetWorldXOffset (Math|Conversions|ToFloat(Integer) (/ (Variables|Default|GetWorldGridWidth) 2)))
  (LocalVariables|SetWorldYOffset (Math|Conversions|ToFloat(Integer) (/ (Variables|Default|GetWorldGridLength) 2)))
  ;[1 1 1] Y Loop
  (for _index (range 0 (- (Variables|Default|GetRow) 1))
    ;[1 1 1] X Loop
    (for _index_2 (range 0 (- (Variables|Default|GetItemPerRow) 1))
      (bind _returnvalue (Game|SpawnActorfromClass (Utilities|Array|Get(acopy) _availableelements (Math|Random|RandomInteger (Utilities|Array|Length _availableelements))) (Math|Transform|MakeTransform (+ (Math|Vector|MakeVector (- (* _index_2 (/ (Math|Conversions|ToFloat(Integer) (Variables|Default|GetWorldGridWidth)) (Math|Conversions|ToFloat(Integer) (- (Variables|Default|GetItemPerRow) 1)))) (LocalVariables|GetWorldXOffset)) (- (* _index (/ (Math|Conversions|ToFloat(Integer) (Variables|Default|GetWorldGridLength)) (Math|Conversions|ToFloat(Integer) (- (Variables|Default|GetRow) 1)))) (LocalVariables|GetWorldYOffset)) 0.0) (Variables|Default|GetWorldLocation))) "AlwaysSpawn" "MultiplyWithRoot" 0 0))
      (Utilities|Array|Add (Variables|Default|GetGridArray) _returnvalue))))