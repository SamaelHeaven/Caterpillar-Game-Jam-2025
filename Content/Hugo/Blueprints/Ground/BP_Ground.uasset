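; BP_Ground is a ground actor that builds a grid over its static mesh through a BPGridComponent.
; On BeginPlay it sets the grid's length and width from the full Y and X extents of the mesh bounds.
; It also passes the root's world location and the mesh's rotation to the component, then calls PopulateGrid.
; The construction script is empty.
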(event EventBeginPlay
  (bind _staticmesh (Variables|Default|GetStaticMesh))
  (bind _boxextent (Collision|GetComponentBounds _staticmesh))
  (Variables|/Game/Hugo/Blueprints/Ground/BP_GridComponent.BP_GridComponent_C|SetWorldGridLength (Variables|Default|GetBP_GridComponent) (* (.y _boxextent) 2.0))
  (Variables|/Game/Hugo/Blueprints/Ground/BP_GridComponent.BP_GridComponent_C|SetWorldGridWidth (Variables|Default|GetBP_GridComponent) (* (.x _boxextent) 2.0))
  (Variables|/Game/Hugo/Blueprints/Ground/BP_GridComponent.BP_GridComponent_C|SetWorldLocation (Variables|Default|GetBP_GridComponent) (Transformation|GetWorldLocation (Variables|Default|GetDefaultSceneRoot)))
  (Variables|/Game/Hugo/Blueprints/Ground/BP_GridComponent.BP_GridComponent_C|SetGroundRotation (Variables|Default|GetBP_GridComponent) (Transformation|GetWorldRotation (Variables|Default|GetStaticMesh)))
  (Default|PopulateGrid (Variables|Default|GetBP_GridComponent)))

(event Collision|EventActorBeginOverlap
  (params (OtherActor :type Actor%20Object%20Reference)))

(event EventTick
  (params (DeltaSeconds :type Float%20%28single-precision%29)))

(fn ConstructionScript)