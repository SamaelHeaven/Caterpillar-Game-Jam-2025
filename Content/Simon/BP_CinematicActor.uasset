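; BP_CinematicActor plays a slideshow intro cinematic that the player advances with the space bar.
; It enables input on begin play, and each press increments an index that swaps the cinematic sprite to the next scene, with a sound cue on one slide.
; The final slide changes the HUD prompt to start the game, and the next press opens MAP_CaterpillarSlide with game-only input and a hidden cursor.
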(event EventBeginPlay
  (Input|EnableInput (Game|GetPlayerController 0)))

(event Input|KeyboardEvents|SpaceBar
  (params (Key :type Key%20Structure :default "None"))
  (bind _returnvalue (Game|GetPlayerController 0))
  (:Pressed
    (bind _output_get (Variables|Default|SetCurrentSpriteIndex (+ (Variables|Default|GetCurrentSpriteIndex) 1)))
    (switch int _output_get
      (:1
        (Variables|Default|SetSpriteToShow "/Game/Simon/IntroTrailerImages/scene3_Sprite.scene3_Sprite")
        (Rendering|Components|Sprite|SetSprite (Variables|Default|GetCinematicSprite) (Variables|Default|GetSpriteToShow) :!label _label))
      (:2
        (Variables|Default|SetSpriteToShow "/Game/Simon/IntroTrailerImages/scene4_Sprite.scene4_Sprite")
        (Audio|PlaySound2D "/Game/Simon/sounds/boo-cue.boo-cue" 1.0 1.0 0.0 0 0)
        (goto _label))
      (:3
        (Variables|Default|SetSpriteToShow "/Game/Simon/IntroTrailerImages/scene5_Sprite.scene5_Sprite")
        (goto _label))
      (:4
        (Variables|Default|SetSpriteToShow "/Game/Simon/IntroTrailerImages/scene6_Sprite.scene6_Sprite")
        (goto _label))
      (:5
        (Variables|Default|SetSpriteToShow "/Game/Simon/IntroTrailerImages/scene7_Sprite.scene7_Sprite")
        (Variables|/Script/UMG.TextBlock|SetText (Variables|/Game/Simon/wbp/WBP_Cinematic.WBP_Cinematic_C|GetTextSpace (Variables|Default|GetHUD)) "[ESPACE]  Commencer")
        (goto _label))
      (:6
        (Game|OpenLevel(byName) "MAP_CaterpillarSlide")
        (Variables|/Script/Engine.PlayerController|SetbShowMouseCursor _returnvalue false)
        (Input|SetInputModeGameOnly _returnvalue false)))))

(fn ConstructionScript)